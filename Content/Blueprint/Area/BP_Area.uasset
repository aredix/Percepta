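; BP_Area is a zone actor that tells the BP_Hitman_Final player which area they are in and which suits are allowed there.
; On begin play it caches the player and its zone enum as a string.
; When the hitman overlaps with a different current area, it updates that area, passes a comma-joined string of allowed suits and plays the UI area animation.
; The box end-overlap only casts to BP_Enemy_Base and does nothing further.
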(event OnComponentEndOverlap(Box)
  (params (OverlappedComponent :type Primitive%20Component%20Object%20Reference) (OtherActor :type Actor%20Object%20Reference) (OtherComp :type Primitive%20Component%20Object%20Reference) (OtherBodyIndex :type Integer))
  (Utilities|Casting|CastToBP_Enemy_Base OtherActor))

(event Custom|UpdateAllowedSuits
  (bind _allowedsuits (Variables|Default|GetAllowedSuits))
  (for (_array_element _array_index) _allowedsuits
    (if (== _array_index 0)
      (Variables|Default|SetCurrentAllowedSuits (Utilities|String|Append (Utilities|String|EnumtoString _array_element) ", "))
      (elif (< _array_index (- (Utilities|Array|Length _allowedsuits) 1))
        (Variables|Default|SetCurrentAllowedSuits (Utilities|String|Append (Variables|Default|GetCurrentAllowedSuits) (Utilities|String|EnumtoString _array_element) ", "))
        (else
          (Variables|Default|SetCurrentAllowedSuits (Utilities|String|Append (Variables|Default|GetCurrentAllowedSuits) (Utilities|String|EnumtoString _array_element))))))))

(event EventBeginPlay
  (bind _asbp_hitman_final (Utilities|Casting|CastToBP_Hitman_Final (Game|GetPlayerCharacter 0)))
  (Variables|Default|SetAs%20BP%20Hitman%20Final _asbp_hitman_final)
  (Variables|Default|SetCurrentZone_String (Utilities|String|EnumtoString (Variables|Default|GetCurrentZone))))

(event Collision|EventActorBeginOverlap
  (params (OtherActor :type Actor%20Object%20Reference))
  (bind _currentzone_string (Variables|Default|GetCurrentZone_String))
  (bind _asbp_hitman_final (Utilities|Casting|CastToBP_Hitman_Final OtherActor))
  (if (Utilities|Enum|NotEqual(Enum) (Variables|/Game/Blueprint/Player/BP_Hitman_Final.BP_Hitman_Final_C|GetCurrentArea _asbp_hitman_final) _currentzone_string)
    (Variables|/Game/Blueprint/Player/BP_Hitman_Final.BP_Hitman_Final_C|SetCurrentArea _asbp_hitman_final _currentzone_string)
    (CallFunction|UpdateAllowedSuits)
    (Variables|/Game/Blueprint/Player/BP_Hitman_Final.BP_Hitman_Final_C|SetAllowedSuits (Variables|Default|GetAs%20BP%20Hitman%20Final) (Variables|Default|GetCurrentAllowedSuits))
    (UserInterface|Animation|PlayAnimation (Variables|/Game/Blueprint/Player/BP_Hitman_Final.BP_Hitman_Final_C|GetUIRef _asbp_hitman_final) (Variables|/Game/Blueprint/UI/Player/WBP_MainInterface.WBP_MainInterface_C|GetAreaAnimation (Variables|/Game/Blueprint/Player/BP_Hitman_Final.BP_Hitman_Final_C|GetUIRef _asbp_hitman_final)) 0.0 1 "Forward" 1.0 false)))

(fn ConstructionScript)