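; BP_SuitChange is an area trigger that changes the hitman character's disguise when it overlaps the zone.
; On overlap it casts to BP_Hitman_Final, swaps the skeletal mesh through ChangeSuit, then stores SuitTarget as the character's CurrentSuit.
; ChangeSuit picks the mesh from SuitChoice by the SuitTarget enum, covering Security, Staff, VIP, BOSS and a default.
; The construction script writes the target suit's name onto the Area text as a label.
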(event Collision|EventActorBeginOverlap
  (params (OtherActor :type Actor%20Object%20Reference))
  (bind _asbp_hitman_final (Utilities|Casting|CastToBP_Hitman_Final OtherActor))
  (bind _output_get (Variables|Default|SetAs%20BP%20Hitman%20Final _asbp_hitman_final))
  (CallFunction|ChangeSuit _output_get)
  (Variables|/Game/Blueprint/Player/BP_Hitman_Final.BP_Hitman_Final_C|SetCurrentSuit _output_get (Variables|Default|GetSuitTarget)))

(fn ConstructionScript
  (Rendering|Components|TextRender|SetText (Variables|Default|GetArea) (Utilities|Text|ToText(String) (Utilities|String|EnumtoString (Variables|Default|GetSuitTarget)))))

(fn ChangeSuit
  (params (Actor :type BP%20Hitman%20Final%20Object%20Reference))
  (switch Utilities|FlowControl|Switch|SwitchonE_Suits (Variables|Default|GetSuitTarget)
    (:NewEnumerator0
      (Components|SkeletalMesh|SetSkeletalMeshAsset (Variables|/Script/Engine.Character|GetMesh Actor) (Utilities|Struct|BreakS_SuitListing (Variables|Default|GetSuitChoice))))
    (:NewEnumerator1
      (Components|SkeletalMesh|SetSkeletalMeshAsset (Variables|/Script/Engine.Character|GetMesh Actor) (Utilities|Struct|BreakS_SuitListing (Variables|Default|GetSuitChoice))))
    (:NewEnumerator2
      (Components|SkeletalMesh|SetSkeletalMeshAsset (Variables|/Script/Engine.Character|GetMesh Actor) (Utilities|Struct|BreakS_SuitListing (Variables|Default|GetSuitChoice))))
    (:NewEnumerator3
      (Components|SkeletalMesh|SetSkeletalMeshAsset (Variables|/Script/Engine.Character|GetMesh Actor) (Utilities|Struct|BreakS_SuitListing (Variables|Default|GetSuitChoice))))
    (:NewEnumerator4
      (Components|SkeletalMesh|SetSkeletalMeshAsset (Variables|/Script/Engine.Character|GetMesh Actor) (Utilities|Struct|BreakS_SuitListing (Variables|Default|GetSuitChoice))))))