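; Interactable boss door that swings open and closed around its yaw axis.
; The Interact event toggles IsClose and plays or reverses a timeline, which offsets the mesh yaw by up to a quarter turn from the rotation saved at BeginPlay.
; A box trigger shows a call-to-action widget while BP_Hitman_Final overlaps it and hides it on exit.
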(event OnComponentBeginOverlap(Box)
  (params (OverlappedComponent :type Primitive%20Component%20Object%20Reference) (OtherActor :type Actor%20Object%20Reference) (OtherComp :type Primitive%20Component%20Object%20Reference) (OtherBodyIndex :type Integer) (bFromSweep :type Boolean) (SweepResult :type Hit%20Result%20Structure%20%28by%20ref%29))
  (Utilities|Casting|CastToBP_Hitman_Final OtherActor)
  (Rendering|SetVisibility (Variables|Default|GetWBP_CallToAction) true false))

(event OnComponentEndOverlap(Box)
  (params (OverlappedComponent :type Primitive%20Component%20Object%20Reference) (OtherActor :type Actor%20Object%20Reference) (OtherComp :type Primitive%20Component%20Object%20Reference) (OtherBodyIndex :type Integer))
  (Utilities|Casting|CastToBP_Hitman_Final OtherActor)
  (Rendering|SetVisibility (Variables|Default|GetWBP_CallToAction) false false))

(event EventInteract
  (bind _sm_bossdoor (Variables|Default|GetSM_BossDoor))
  (bind _relativerotation (Variables|/Script/Engine.SceneComponent|GetRelativeRotation _sm_bossdoor))
  (if (Variables|Default|GetisClose)
    (Variables|Default|SetisClose false)
    (bind _value (Timeline|Timeline Play)
      (:Update
        (Transformation|SetRelativeRotation _sm_bossdoor (Math|Rotator|MakeRotator (.roll _relativerotation) (.pitch _relativerotation) (+ (* _value 9e+01) (.yaw (Variables|Default|GetOriginRotation)))) false false)))
    (else
      (Variables|Default|SetisClose true)
      (Timeline|Timeline Reverse))))

(event EventBeginPlay
  (Variables|Default|SetOriginRotation (Variables|/Script/Engine.SceneComponent|GetRelativeRotation (Variables|Default|GetSM_BossDoor))))

(fn ConstructionScript)