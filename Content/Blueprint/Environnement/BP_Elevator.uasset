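; Elevator actor with two sliding doors and a cabin that travels between the lobby and one upper level.
; An outer trigger overlap toggles the doors, while an inner one closes them and polls CanMove with delays before moving the cabin.
; Timelines offset doors and cabin from positions cached at BeginPlay, playing or reversing for each direction.
; Doors block movement while animating and reopen when cabin travel finishes.
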(event OnComponentBeginOverlap(CB_Detection_Out)
  (params (OverlappedComponent :type Primitive%20Component%20Object%20Reference) (OtherActor :type Actor%20Object%20Reference) (OtherComp :type Primitive%20Component%20Object%20Reference) (OtherBodyIndex :type Integer) (bFromSweep :type Boolean) (SweepResult :type Hit%20Result%20Structure%20%28by%20ref%29))
  (if (Variables|Default|GetisDoorClosed)
    (CallFunction|UpdateDoorState true)
    (else
      (CallFunction|UpdateDoorState false))))

(event OnComponentBeginOverlap(CB_Detection_In)
  (params (OverlappedComponent :type Primitive%20Component%20Object%20Reference) (OtherActor :type Actor%20Object%20Reference) (OtherComp :type Primitive%20Component%20Object%20Reference) (OtherBodyIndex :type Integer) (bFromSweep :type Boolean) (SweepResult :type Hit%20Result%20Structure%20%28by%20ref%29))
  (CallFunction|UpdateDoorState false)
  (if (Variables|Default|GetCanMove) :!label _label
    (Utilities|FlowControl|Delay 2.0)
    (CallFunction|ElevatorUpandDown (Variables|Default|GetIsAtLobby))
    (else
      (Utilities|FlowControl|Delay 2.0)
      (goto _label))))

(event Custom|UpdateDoorState
  (params (Open :type Boolean))
  (bind _sm_porte_gauche (Variables|Default|GetSM_Porte_Gauche))
  (bind _sm_porte_droite (Variables|Default|GetSM_Porte_Droite))
  (bind _relativelocation (Variables|/Script/Engine.SceneComponent|GetRelativeLocation _sm_porte_droite))
  (bind _relativelocation_2 (Variables|/Script/Engine.SceneComponent|GetRelativeLocation _sm_porte_gauche))
  (if Open
    (Variables|Default|SetisDoorClosed false)
    (bind _value (Timeline|OpenCloseDoor Play)
      (:Update
        (Variables|Default|SetCanMove false)
        (Transformation|SetRelativeLocation _sm_porte_gauche (Math|Vector|MakeVector (+ (.x (Variables|Default|GetOriginDoorG)) (* _value 7e+01)) (.y _relativelocation_2) (.z _relativelocation_2)) false false)
        (Transformation|SetRelativeLocation _sm_porte_droite (Math|Vector|MakeVector (- (.x (Variables|Default|GetOriginDoorD)) (* _value 7e+01)) (.y _relativelocation) (.z _relativelocation)) false false))
      (:Finished
        (Variables|Default|SetCanMove true)))
    (else
      (Variables|Default|SetisDoorClosed true)
      (Timeline|OpenCloseDoor Reverse))))

(event Custom|Elevator%20Up%20and%20Down
  (params (Up? :type Boolean))
  (bind _sm_cabine (Variables|Default|GetSM_Cabine))
  (bind _relativelocation (Variables|/Script/Engine.SceneComponent|GetRelativeLocation _sm_cabine))
  (if Up?
    (Variables|Default|SetIsAtLobby false)
    (bind _value (Timeline|Up%20and%20Down Play)
      (:Update
        (Transformation|SetRelativeLocation _sm_cabine (Math|Vector|MakeVector (.x _relativelocation) (.y _relativelocation) (+ (* _value 6e+02) (.z (Variables|Default|GetOriginCabine)))) false false))
      (:Finished
        (CallFunction|UpdateDoorState true)))
    (else
      (Variables|Default|SetIsAtLobby true)
      (Timeline|Up%20and%20Down Reverse))))

(event EventBeginPlay
  (Variables|Default|SetOriginDoorG (Variables|/Script/Engine.SceneComponent|GetRelativeLocation (Variables|Default|GetSM_Porte_Gauche)))
  (Variables|Default|SetOriginDoorD (Variables|/Script/Engine.SceneComponent|GetRelativeLocation (Variables|Default|GetSM_Porte_Droite)))
  (Variables|Default|SetOriginCabine (Variables|/Script/Engine.SceneComponent|GetRelativeLocation (Variables|Default|GetSM_Cabine))))

(fn ConstructionScript)