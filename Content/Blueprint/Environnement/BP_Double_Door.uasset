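; Interactable double door that the player's Hitman character can open, with no logic to close it again.
; Interact plays a timeline that swings both leaves 90 degrees in opposite directions from their starting yaw, then clears IsClose and hides the prompt.
; A box overlap shows the call-to-action widget while the Hitman is inside and the door is closed.
; Tick rotates that widget to face the player's follow camera.
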(event OnComponentBeginOverlap(Box)
  (params (OverlappedComponent :type Primitive%20Component%20Object%20Reference) (OtherActor :type Actor%20Object%20Reference) (OtherComp :type Primitive%20Component%20Object%20Reference) (OtherBodyIndex :type Integer) (bFromSweep :type Boolean) (SweepResult :type Hit%20Result%20Structure%20%28by%20ref%29))
  (Utilities|Casting|CastToBP_Hitman_Final OtherActor)
  (if (Variables|Default|GetisClose)
    (Rendering|SetVisibility (Variables|Default|GetWBP_CallToAction) true false)))

(event OnComponentEndOverlap(Box)
  (params (OverlappedComponent :type Primitive%20Component%20Object%20Reference) (OtherActor :type Actor%20Object%20Reference) (OtherComp :type Primitive%20Component%20Object%20Reference) (OtherBodyIndex :type Integer))
  (Utilities|Casting|CastToBP_Hitman_Final OtherActor)
  (Rendering|SetVisibility (Variables|Default|GetWBP_CallToAction) false false))

(event EventTick
  (params (DeltaSeconds :type Float%20%28single-precision%29))
  (bind _wbp_calltoaction (Variables|Default|GetWBP_CallToAction))
  (Transformation|SetWorldRotation _wbp_calltoaction (Math|Rotator|FindLookatRotation (Transformation|GetWorldLocation _wbp_calltoaction) (Transformation|GetWorldLocation (Variables|/Game/Blueprint/Player/BP_Hitman_Final.BP_Hitman_Final_C|GetFollowCamera (Variables|Default|GetAs%20BP%20Hitman%20Final)))) false false))

(event EventInteract
  (bind _sm_big_door_droite (Variables|Default|GetSM_Big_Door_Droite))
  (bind _sm_big_door_gauche (Variables|Default|GetSM_Big_Door_Gauche))
  (bind _relativerotation (Variables|/Script/Engine.SceneComponent|GetRelativeRotation _sm_big_door_droite))
  (bind _relativerotation_2 (Variables|/Script/Engine.SceneComponent|GetRelativeRotation _sm_big_door_gauche))
  (if (Variables|Default|GetisClose)
    (bind _value (Timeline|Timeline Play)
      (:Update
        (Transformation|SetRelativeRotation _sm_big_door_droite (Math|Rotator|MakeRotator (.roll _relativerotation) (.pitch _relativerotation) (+ (* _value 9e+01) (.yaw (Variables|Default|GetOriginRotationD)))) false false)
        (Transformation|SetRelativeRotation _sm_big_door_gauche (Math|Rotator|MakeRotator (.roll _relativerotation_2) (.pitch _relativerotation_2) (+ (* _value -9e+01) (.yaw (Variables|Default|GetOriginRotationG)))) false false)
        (Rendering|SetVisibility (Variables|Default|GetWBP_CallToAction) false false)
        (Variables|Default|SetisClose false)))))

(event EventBeginPlay
  (Variables|Default|SetOriginRotationG (Variables|/Script/Engine.SceneComponent|GetRelativeRotation (Variables|Default|GetSM_Big_Door_Gauche)))
  (Variables|Default|SetOriginRotationD (Variables|/Script/Engine.SceneComponent|GetRelativeRotation (Variables|Default|GetSM_Big_Door_Droite)))
  (bind _asbp_hitman_final (Utilities|Casting|CastToBP_Hitman_Final (Game|Player|GetPlayerPawn 0)))
  (Variables|Default|SetAs%20BP%20Hitman%20Final _asbp_hitman_final))

(fn ConstructionScript)