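; Interactive hinged door that swings open and shut, with a call-to-action widget shown while the player is in its trigger box.
; Interact toggles IsClose and plays or reverses a timeline that yaws the mesh 90 degrees, disabling collision during the swing.
; Enemies entering or leaving the box trigger the interaction automatically.
; When the swing finishes during objective 6, the Target's timing flag copies the closed state; Tick prints that state for debugging.
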(event OnComponentBeginOverlap(Box)
  (params (OverlappedComponent :type Primitive%20Component%20Object%20Reference) (OtherActor :type Actor%20Object%20Reference) (OtherComp :type Primitive%20Component%20Object%20Reference) (OtherBodyIndex :type Integer) (bFromSweep :type Boolean) (SweepResult :type Hit%20Result%20Structure%20%28by%20ref%29))
  (Utilities|FlowControl|Sequence
    (:then_0
      (CallFunction|PlayerDisplayCalltoAction OtherActor))
    (:then_1
      (CallFunction|IACheck OtherActor))))

(event OnComponentEndOverlap(Box)
  (params (OverlappedComponent :type Primitive%20Component%20Object%20Reference) (OtherActor :type Actor%20Object%20Reference) (OtherComp :type Primitive%20Component%20Object%20Reference) (OtherBodyIndex :type Integer))
  (Utilities|FlowControl|Sequence
    (:then_0
      (CallFunction|PlayerHideCalltoAction OtherActor))
    (:then_1
      (CallFunction|IACheck OtherActor))))

(event EventBeginPlay
  (Variables|Default|SetOriginRotation (Variables|/Script/Engine.SceneComponent|GetRelativeRotation (Variables|Default|GetSM_Door))))

(event EventTick
  (params (DeltaSeconds :type Float%20%28single-precision%29))
  (Development|PrintString (Utilities|String|Append "The Door is : " (Utilities|String|ToString(Boolean) (Variables|Default|GetisClose))) true true "(R=0.000000,G=0.660000,B=1.000000,A=1.000000)" 0.0))

(event EventInteract
  (bind _sm_door (Variables|Default|GetSM_Door))
  (bind _relativerotation (Variables|/Script/Engine.SceneComponent|GetRelativeRotation _sm_door))
  (Collision|SetCollisionEnabled (Variables|Default|GetSM_Door) "NoCollision")
  (if (Variables|Default|GetisClose)
    (Variables|Default|SetisClose false)
    (bind _value (Timeline|OpenClose Play)
      (:Update
        (Transformation|SetRelativeRotation _sm_door (Math|Rotator|MakeRotator (.roll _relativerotation) (.pitch _relativerotation) (+ (* _value 9e+01) (.yaw (Variables|Default|GetOriginRotation)))) false false))
      (:Finished
        (Collision|SetCollisionEnabled (Variables|Default|GetSM_Door) "QueryAndPhysics")
        (if (== (Variables|/Game/Blueprint/Player/BP_Hitman_Final.BP_Hitman_Final_C|GetCurrentObjectifIndex (.AsBP%20Hitman%20Final (Utilities|Casting|CastToBP_Hitman_Final (Game|GetPlayerCharacter 0)))) 6)
          (Variables|/Game/Blueprint/IA/BP_Enemy_Base.BP_Enemy_Base_C|SetIsInRightTiming (Variables|Default|GetTarget) (Variables|Default|GetisClose)))))
    (else
      (Variables|Default|SetisClose true)
      (Timeline|OpenClose Reverse))))

(fn ConstructionScript)

(fn PlayerDisplayCalltoAction
  (params (Object :type Object%20Object%20Reference))
  (Utilities|Casting|CastToBP_Hitman_Final Object)
  (Rendering|SetVisibility (Variables|Default|GetWBP_CallToAction) true false))

(fn IACheck
  (params (Object :type Object%20Object%20Reference))
  (Utilities|Casting|CastToBP_Enemy_Base Object)
  (Class|BPIInteract|Interact(Message) self))

(fn PlayerHideCalltoAction
  (params (Object :type Object%20Object%20Reference))
  (Utilities|Casting|CastToBP_Hitman_Final Object)
  (Rendering|SetVisibility (Variables|Default|GetWBP_CallToAction) false false))