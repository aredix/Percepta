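; Interactable distributor world event for the Hitman player that lures chaser enemy AI to a reach point.
; At BeginPlay it caches chaser AI controllers, from all enemies or a specified list.
; Interact, gated by suit and objective, sets their Blackboard event location and flags, then advances the objective.
; Enemies overlapping the reach box trigger the event's end; a toggleable prompt plane yaws toward the player.
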(event OnComponentBeginOverlap(ReachPointBox)
  (params (OverlappedComponent :type Primitive%20Component%20Object%20Reference) (OtherActor :type Actor%20Object%20Reference) (OtherComp :type Primitive%20Component%20Object%20Reference) (OtherBodyIndex :type Integer) (bFromSweep :type Boolean) (SweepResult :type Hit%20Result%20Structure%20%28by%20ref%29))
  (bind _returnvalue (Game|GetPlayerCharacter 0))
  (bind _asbp_hitman_final (Utilities|Casting|CastToBP_Hitman_Final _returnvalue))
  (bind _currentobjectifindex (Variables|/Game/Blueprint/Player/BP_Hitman_Final.BP_Hitman_Final_C|GetCurrentObjectifIndex _asbp_hitman_final))
  (bind _asbp_enemy_base (Utilities|Casting|CastToBP_Enemy_Base OtherActor))
  (if (and (ScalableFloat|GetValueasBool (AI|GetBlackboard (AI|GetAIController _asbp_enemy_base)) (Variables|Default|GetWorldEventState)) (or (== 3 _currentobjectifindex) (== _currentobjectifindex 4)))
    (Default|TriggerEndWorldEvent1 _asbp_enemy_base (Variables|Default|GetWaitingTime) (Variables|Default|GetWorldEventValue) (Variables|Default|GetReturnToDefaultLocationValue) (Variables|Default|GetTarget))))

(event EventInteract
  (bind _asbp_hitman_final (Utilities|Casting|CastToBP_Hitman_Final (Game|GetPlayerCharacter 0)))
  (if (and (Utilities|Enum|Equal(Enum) (Variables|/Game/Blueprint/Player/BP_Hitman_Final.BP_Hitman_Final_C|GetCurrentSuit _asbp_hitman_final) "NewEnumerator1") (== (Variables|/Game/Blueprint/Player/BP_Hitman_Final.BP_Hitman_Final_C|GetCurrentObjectifIndex _asbp_hitman_final) 2))
    (for _array_element (Variables|Default|GetAIToMove)
      (bind _blackboard (Variables|/Script/AIModule.AIController|GetBlackboard _array_element)
        (:then
          (AI|Components|Blackboard|SetValueasVector _blackboard (Variables|Default|GetWorldEvent1_Location) (Transformation|GetWorldLocation (Variables|Default|GetReachPointBox)))
          (AI|Components|Blackboard|SetValueasBool _blackboard (Variables|Default|GetWorldEvent1) true)
          (AI|Components|Blackboard|SetValueasBool _blackboard (Variables|Default|GetChaserNPC) true))
        (:else)))
    (if (== (Variables|/Game/Blueprint/Player/BP_Hitman_Final.BP_Hitman_Final_C|GetCurrentObjectifIndex (Variables|Default|GetAs%20BP%20Hitman%20Final)) 2)
      (bind _as_bp_hitman_final (Variables|Default|GetAs%20BP%20Hitman%20Final)
        (:then
          (Math|Integer|IncrementInt (Variables|/Game/Blueprint/Player/BP_Hitman_Final.BP_Hitman_Final_C|GetCurrentObjectifIndex _as_bp_hitman_final)
            (:%20%20
              (Default|UpdateObjectif _as_bp_hitman_final)
              (Variables|/Game/Blueprint/IA/BP_Enemy_Base.BP_Enemy_Base_C|SetIsInRightTiming (Variables|Default|GetTarget) true))))
        (:else)))))

(event Collision|EventActorBeginOverlap
  (params (OtherActor :type Actor%20Object%20Reference))
  (|CallParentFunction OtherActor) ; This node is disabled and will not be called.\nDrag off pins to build functionality.
)

(event EventHideUI
  (bind _plane (Variables|Default|GetPlane))
  (Rendering|SetVisibility _plane false false)
  (Components|Tick|SetComponentTickEnabled _plane false))

(event EventTick
  (params (DeltaSeconds :type Float%20%28single-precision%29))
  (bind _plane (Variables|Default|GetPlane))
  (Transformation|SetWorldRotation _plane (Math|Rotator|MakeRotator -9e+01 1.8e+02 (+ (.yaw (Math|Rotator|FindLookatRotation (Transformation|GetWorldLocation _plane) (Transformation|GetWorldLocation (Variables|/Script/Engine.Character|GetMesh (.AsBP%20Hitman%20Final (Utilities|Casting|CastToBP_Hitman_Final (Game|GetPlayerCharacter 0))))))) 9e+01)) false false))

(event EventBeginPlay
  (Utilities|FlowControl|Sequence
    (:then_0
      (bind _asbp_hitman_final (Utilities|Casting|CastToBP_Hitman_Final (Game|GetPlayerCharacter 0)))
      (Variables|Default|SetAs%20BP%20Hitman%20Final _asbp_hitman_final))
    (:then_1
      (Utilities|Array|Clear (Variables|Default|GetAIToMove))
      (if (Variables|Default|GetisGlobalToAllAI)
        (bind _outactors (Actor|GetAllActorsOfClass "/Game/Blueprint/IA/BP_Enemy_Base.BP_Enemy_Base_C"))
        (for _array_element _outactors
          (bind _asaic_enemy_base_v2 (Utilities|Casting|CastToAIC_Enemy_BaseV2 (AI|GetAIController _array_element)))
          (if (Variables|/Game/Blueprint/IA/BP_Enemy_Base.BP_Enemy_Base_C|GetChaserNPC _array_element)
            (Utilities|Array|Add (Variables|Default|GetAIToMove) _asaic_enemy_base_v2)))
        (else
          (for _array_element_2 (Variables|Default|GetSpecificAI_To_Move)
            (bind _asaic_enemy_base_v2_2 (Utilities|Casting|CastToAIC_Enemy_BaseV2 (AI|GetAIController _array_element_2)))
            (if (Variables|/Game/Blueprint/IA/BP_Enemy_Base.BP_Enemy_Base_C|GetChaserNPC _array_element_2)
              (Utilities|Array|Add (Variables|Default|GetAIToMove) _asaic_enemy_base_v2_2))))))))

(event EventDisplayUI
  (bind _plane (Variables|Default|GetPlane))
  (Rendering|SetVisibility _plane true false)
  (Components|Tick|SetComponentTickEnabled _plane true))

(fn ConstructionScript
  (|CallParentFunction))