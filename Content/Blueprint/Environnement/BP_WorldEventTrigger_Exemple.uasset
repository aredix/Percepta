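; Example interactable world event trigger that, when the player wears a specific suit at the right objective step, alerts chaser NPCs and advances the objective.
; BeginPlay caches the player and the AI controllers of enemies flagged as ChaserNPC.
; Interact sets their WorldEvent1 and ChaserNPC Blackboard keys, updates the objective and flags Target as in the right timing.
; DisplayInteract reveals a plane.
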(event Custom|Display%20Interact
  (Rendering|SetVisibility (Variables|Default|GetPlane) true false))

(event Collision|EventActorBeginOverlap
  (params (OtherActor :type Actor%20Object%20Reference)))

(event EventTick
  (params (DeltaSeconds :type Float%20%28single-precision%29)))

(event EventInteract
  (bind _asbp_hitman_final (Utilities|Casting|CastToBP_Hitman_Final (Game|GetPlayerCharacter 0)))
  (if (and (Utilities|Enum|Equal(Enum) (Variables|/Game/Blueprint/Player/BP_Hitman_Final.BP_Hitman_Final_C|GetCurrentSuit _asbp_hitman_final) "NewEnumerator1") (== (Variables|/Game/Blueprint/Player/BP_Hitman_Final.BP_Hitman_Final_C|GetCurrentObjectifIndex _asbp_hitman_final) 2))
    (for _array_element (Variables|Default|GetAll_AIC_Ref)
      (bind _blackboard (Variables|/Script/AIModule.AIController|GetBlackboard _array_element)
        (:then
          (AI|Components|Blackboard|SetValueasBool _blackboard (Variables|Default|GetWorldEvent1) true)
          (AI|Components|Blackboard|SetValueasBool _blackboard (Variables|Default|GetChaserNPC) true))
        (:else)))
    (if (== (Variables|/Game/Blueprint/Player/BP_Hitman_Final.BP_Hitman_Final_C|GetCurrentObjectifIndex (Variables|Default|GetAs%20BP%20Hitman%20Final)) 2)
      (bind _as_bp_hitman_final (Variables|Default|GetAs%20BP%20Hitman%20Final)
        (:then
          (Math|Integer|IncrementInt (Variables|/Game/Blueprint/Player/BP_Hitman_Final.BP_Hitman_Final_C|GetCurrentObjectifIndex _as_bp_hitman_final)
            (:%20%20
              (Default|UpdateObjectif _as_bp_hitman_final)
              (Variables|/Game/Blueprint/IA/BP_Enemy_Base.BP_Enemy_Base_C|SetIsInRightTiming (Variables|Default|GetTarget) true))))
        (:else)))))

(event EventBeginPlay
  (Utilities|FlowControl|Sequence
    (:then_0
      (Utilities|Array|Clear (Variables|Default|GetAll_AIC_Ref)))
    (:then_1
      (bind _outactors (Actor|GetAllActorsOfClass "/Game/Blueprint/IA/BP_Enemy_Base.BP_Enemy_Base_C"))
      (for _array_element _outactors
        (bind _asaic_enemy_base_v2 (Utilities|Casting|CastToAIC_Enemy_BaseV2 (AI|GetAIController _array_element)))
        (if (Variables|/Game/Blueprint/IA/BP_Enemy_Base.BP_Enemy_Base_C|GetChaserNPC _array_element)
          (Utilities|Array|Add (Variables|Default|GetAll_AIC_Ref) _asaic_enemy_base_v2))))
    (:then_2
      (bind _asbp_hitman_final (Utilities|Casting|CastToBP_Hitman_Final (Game|GetPlayerCharacter 0)))
      (Variables|Default|SetAs%20BP%20Hitman%20Final _asbp_hitman_final))))

(fn ConstructionScript)