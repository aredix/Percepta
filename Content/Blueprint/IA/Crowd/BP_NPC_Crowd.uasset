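; Crowd NPC Blueprint that gives each instance a random look and a looping animation.
; On BeginPlay it waits a random sub-second delay to stagger instances, then applies a random skeletal mesh from MeshToApply.
; It picks one of the first ten MontageToPlay entries and replays that same montage on each blend out, so the animation is randomized only once per instance.
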(event Custom|PlayRandomAnimation
  (params (value :type Integer))
  (Animation|Montage|PlayMontage (Variables|Character|GetMesh) (Utilities|Array|Get(acopy) (Variables|Default|GetMontage%20to%20Play) value) 1.0 0.5
    (:OnBlendOut
      (CallFunction|PlayRandomAnimation (Variables|Default|GetCurrentAnimIndex)))))

(event EventBeginPlay
  (bind _meshtoapply (Variables|Default|GetMeshToApply))
  (|CallParentFunction)
  (Utilities|FlowControl|Delay (Math|Random|RandomFloatinRange 0.0 1.0))
  (Components|SkeletalMesh|SetSkeletalMeshAsset (Variables|Character|GetMesh) (Utilities|Array|Get(acopy) _meshtoapply (Math|Random|RandomIntegerinRange 0 (- (Utilities|Array|Length _meshtoapply) 1))))
  (bind _output_get (Variables|Default|SetCurrentAnimIndex (Math|Random|RandomIntegerinRange 0 9)))
  (CallFunction|PlayRandomAnimation _output_get))

(fn ConstructionScript
  (|CallParentFunction))