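; BP_FX_Fountain is a casino fountain effect that fires fifteen particle components in a timed, repeating sequence.
; On BeginPlay it activates the first jet after a short delay, then steps through right and left arrays of seven jets simultaneously.
; A delayed for-loop macro spaces each activation by TimeDelay, and completion of the left-side loop restarts the whole cycle.
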(event EventBeginPlay
  (Variables|Default|SetParticles_R (Utilities|Array|MakeArray (Variables|Default|GetP_Fountain_02) (Variables|Default|GetP_Fountain_03) (Variables|Default|GetP_Fountain_04) (Variables|Default|GetP_Fountain_05) (Variables|Default|GetP_Fountain_06) (Variables|Default|GetP_Fountain_07) (Variables|Default|GetP_Fountain_08)))
  (Variables|Default|SetParticles_L (Utilities|Array|MakeArray (Variables|Default|GetP_Fountain_09) (Variables|Default|GetP_Fountain_10) (Variables|Default|GetP_Fountain_11) (Variables|Default|GetP_Fountain_12) (Variables|Default|GetP_Fountain_13) (Variables|Default|GetP_Fountain_14) (Variables|Default|GetP_Fountain_15)))
  (Utilities|FlowControl|Delay 1.6 :!label _label)
  (Components|Activation|Activate (Variables|Default|GetP_Fountain_01) true)
  (Utilities|FlowControl|Delay (Variables|Default|GetTime_Delay))
  (Utilities|FlowControl|Sequence
    (:then_0
      (bind _arrayelement (Utilities|ForloopwithDelay (Variables|Default|GetTime_Delay) (Variables|Default|GetParticles_R))
        (:Body
          (Components|Activation|Activate _arrayelement true))))
    (:then_1
      (bind _arrayelement_2 (Utilities|ForloopwithDelay (Variables|Default|GetTime_Delay) (Variables|Default|GetParticles_L))
        (:Body
          (Components|Activation|Activate _arrayelement_2 true))
        (:Completed
          (goto _label))))))

(fn ConstructionScript)