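; BP_FX_Fountain_Rotation is a casino fountain effect that fires its particle components in sequence on an endless cycle.
; On BeginPlay it gathers thirteen fountain particle components into an array, then waits briefly before each pass.
; A custom for-loop-with-delay macro reactivates each component with a reset, spaced by TimeDelay, and its completion restarts the cycle.
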(event EventBeginPlay
  (Variables|Default|SetParticles_Rotate (Utilities|Array|MakeArray (Variables|Default|GetP_Fountain_02) (Variables|Default|GetP_Fountain_03) (Variables|Default|GetP_Fountain_04) (Variables|Default|GetP_Fountain_05) (Variables|Default|GetP_Fountain_06) (Variables|Default|GetP_Fountain_07) (Variables|Default|GetP_Fountain_08) (Variables|Default|GetP_Fountain_09) (Variables|Default|GetP_Fountain_10) (Variables|Default|GetP_Fountain_11) (Variables|Default|GetP_Fountain_12) (Variables|Default|GetP_Fountain_13) (Variables|Default|GetP_Fountain_14)))
  (Utilities|FlowControl|Delay 1.6 :!label _label)
  (bind _arrayelement (Utilities|ForloopwithDelay (Variables|Default|GetTime_Delay) (Variables|Default|GetParticles_Rotate))
    (:Body
      (Components|Activation|Activate _arrayelement true))
    (:Completed
      (goto _label))))

(fn ConstructionScript)