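; BP_Prop_Slot_Machine_02 is a casino slot machine prop with five rotating cylinder meshes.
; On BeginPlay it binds a separate RotatingMovement component to each cylinder, so the cylinders rotate independently of the rest of the actor.
; The graph has no spin, stop or payout logic, and the construction script is empty.
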(event EventBeginPlay
  (Components|Movement|SetUpdatedComponent (Variables|Default|GetRotatingMovement) (Variables|Default|GetSM_Prop_Slot_Machine_03_Cylinder_01))
  (Components|Movement|SetUpdatedComponent (Variables|Default|GetRotatingMovement1) (Variables|Default|GetSM_Prop_Slot_Machine_03_Cylinder_02))
  (Components|Movement|SetUpdatedComponent (Variables|Default|GetRotatingMovement2) (Variables|Default|GetSM_Prop_Slot_Machine_03_Cylinder_03))
  (Components|Movement|SetUpdatedComponent (Variables|Default|GetRotatingMovement3) (Variables|Default|GetSM_Prop_Slot_Machine_03_Cylinder_04))
  (Components|Movement|SetUpdatedComponent (Variables|Default|GetRotatingMovement4) (Variables|Default|GetSM_Prop_Slot_Machine_03_Cylinder_05)))

(fn ConstructionScript)